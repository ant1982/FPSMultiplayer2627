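; Cookable frag grenade lethal item that turns a held grenade into a thrown, dropped or in-hand explosion.
; Activation starts a fuse timer and shows a cooking widget.
; Release spawns BP_FragGrenade ahead of the camera with the remaining fuse, while dropping or expiry spawns it at the TPP component.
; The server spawn event pitches it above control rotation and reduces lethal ammo through the owner's inventory component.
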(event Custom|ExplodeGrenade
  ;[0 0 0] Activate
  (if (not (Variables|Default|GetbReleased))
    (Widget|RemovefromParent (Variables|Default|GetCookingGrenadeWidget))
    (CallFunction|ServerSpawnGrenade 0.01 (Transformation|GetWorldLocation (Variables|Default|GetTPP)))))

(event Custom|Server_SpawnGrenade
  (params (TimeLeft :type Float%20%28double-precision%29) (Spawn%20Transform%20Location :type Vector))
  (bind _returnvalue (Components|GetOwner))
  (bind _returnvalue_2 (Components|GetOwner))
  (bind _returnvalue_3 (Actor|GetComponentbyClass _returnvalue "/Game/FPS/Blueprints/BlueprintsComponents/AC_InventorySystem.AC_InventorySystem_C"))
  (bind _returnvalue_4 (Game|GetInstigatorController _returnvalue_2))
  (bind _returnvalue_5 (Pawn|GetControlRotation _returnvalue_4 :!class /Script/Engine.Controller))
  ;[0.15 0 0] Sever Spawn Grenade
  (bind _returnvalue_6 (Game|SpawnActorfromClass "/Game/FPS/Blueprints/Grenade/BP_FragGrenade.BP_FragGrenade_C" (Math|Transform|MakeTransform Spawn%20Transform%20Location (Math|Rotator|MakeRotator (.roll _returnvalue_5) (+ (.pitch _returnvalue_5) 15.0) (.yaw _returnvalue_5)) "1.000000,1.000000,1.000000") "Undefined" "OverrideRootScale" _returnvalue_4 TimeLeft 0.0 (.AsPawn (Utilities|Casting|CastToPawn _returnvalue_2))))
  (Utilities|IsValid _returnvalue_6
    (:Is%20Valid
      (Utilities|IsValid _returnvalue_3
        (:Is%20Valid
          (Default|ReduceLethalAmmo _returnvalue_3))))))

(event Custom|Reset
  ;[0 0 0] Reset
  (Variables|Default|SetbReleased false)
  (Utilities|Time|ClearandInvalidateTimerbyHandle (Variables|Default|GetCookGrenadeTimer)))

(event EventActivate
  ;[0 0 0] Activate
  (CallFunction|Reset)
  (bind _returnvalue (Utilities|Time|SetTimerbyEvent (delegate Custom|ExplodeGrenade) (Variables|Default|GetTimeToExplode)))
  (Variables|Default|SetCookGrenadeTimer _returnvalue)
  (bind _returnvalue_2 (UserInterface|CreateWidget "/Game/FPS/UI/Gameplay/WB_CookingGrenade.WB_CookingGrenade_C" (Game|GetPlayerController 0)))
  (bind _output_get (Variables|Default|SetCookingGrenadeWidget _returnvalue_2))
  (UserInterface|Viewport|AddtoViewport _output_get 0))

(event EventDropLethal
  (bind _cookgrenadetimer (Variables|Default|GetCookGrenadeTimer))
  ;[0 0 0] Drop Lethal
  (Variables|Default|SetbReleased true)
  (if (Utilities|Time|IsTimerActivebyHandle _cookgrenadetimer)
    (CallFunction|ServerSpawnGrenade (Utilities|Time|GetTimerRemainingTimebyHandle _cookgrenadetimer) (Transformation|GetWorldLocation (Variables|Default|GetTPP)))
    (Utilities|Time|ClearandInvalidateTimerbyHandle _cookgrenadetimer)))

(event EventOnRelease
  ;[0 0 0] On release
  (bind _cookinggrenadewidget (Variables|Default|GetCookingGrenadeWidget)
    (:then
      (Widget|RemovefromParent _cookinggrenadewidget)
      (Variables|Default|SetbReleased true)
      (Utilities|Time|ClearandInvalidateTimerbyHandle (Variables|Default|GetCookGrenadeTimer)))
    (:else)))

(event EventReleaseLethal
  ;[0 0 0] Release
  (bind _asplayer_controller (Utilities|Casting|CastToPlayerController (Game|GetInstigatorController (Components|GetOwner))))
  (CallFunction|ServerSpawnGrenade (Utilities|Time|GetTimerRemainingTimebyHandle (Variables|Default|GetCookGrenadeTimer)) (Math|Vector|MakeVector (.X (Math|Vector|BreakVector (+ (Camera|GetCameraLocation (Variables|/Script/Engine.PlayerController|GetPlayerCameraManager _asplayer_controller)) (* (Transformation|GetActorForwardVector _asplayer_controller) 1e+02)))) (.Y (Math|Vector|BreakVector (+ (Camera|GetCameraLocation (Variables|/Script/Engine.PlayerController|GetPlayerCameraManager _asplayer_controller)) (* (Transformation|GetActorForwardVector _asplayer_controller) 1e+02)))) (+ (.Z (Math|Vector|BreakVector (+ (Camera|GetCameraLocation (Variables|/Script/Engine.PlayerController|GetPlayerCameraManager _asplayer_controller)) (* (Transformation|GetActorForwardVector _asplayer_controller) 1e+02)))) 3e+01))))

(fn ConstructionScript
  (|CallParentFunction)
  (Variables|Default|SetUI_Icon "/Game/FPS/UI/Textures/T_FragGrenadeIcon.T_FragGrenadeIcon"))