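; BP_PreviewLethal is a preview actor that shows the lethal item from the player's preview loadout.
; On BeginPlay it retries every 0.1 seconds until the player controller is valid, then binds to the AC_Loadout component's preview-loadout-changed event.
; Each change fetches the preview loadout, async loads its lethal mesh and applies it to the LethalMesh static mesh component.
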(event Custom|SetNewPreviewLoadout
  ;[0 0 0] Update Attachments
  (Variables|Default|SetPreview%20Loadout (Default|GetPreviewLoadout (Variables|Default|GetLoadoutComponent)))
  (CallFunction|UpdateWeapon))

(event Custom|UpdateWeapon
  (bind _preview_loadout (Variables|Default|GetPreview%20Loadout))
  (bind _lethalmesh (Variables|/Game/FPS/Blueprints/DataAssets/Lethal/PDA_LethalEquipment.PDA_LethalEquipment_C|GetLethalMesh (.lethal _preview_loadout)))
  ;[0 0 0] Update Weapon
  (Utilities|AsyncLoadAsset _lethalmesh
    (:Completed
      (Components|StaticMesh|SetStaticMesh (Variables|Default|GetLethalMesh) (Utilities|ResolveSoftReference _lethalmesh)))))

(event Custom|PreviewLoadoutChanged_Event
  ;[0 0 0] Begin play
  (CallFunction|SetNewPreviewLoadout))

(event EventBeginPlay
  (bind _returnvalue (Game|GetPlayerController 0))
  ;[0 0 0] Begin play
  (Utilities|IsValid _returnvalue :!label _label ; ensure that the controller is valid
    (:Is%20Valid
      (bind _output_get (Variables|Default|SetController _returnvalue))
      (Variables|Default|SetLoadoutComponent 0)
      (EventDispatchers|BindEventtoPreviewLoadoutChanged (Actor|GetComponentbyClass _output_get "/Game/FPS/Blueprints/BlueprintsComponents/AC_Loadout.AC_Loadout_C") (delegate Custom|PreviewLoadoutChanged_Event)))
    (:Is%20Not%20Valid
      (Utilities|FlowControl|Delay 0.1)
      (goto _label))))

(fn ConstructionScript)