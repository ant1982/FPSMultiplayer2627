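; Base magazine attachment for FPS weapons, with separate first-person (FPP) and third-person (TPP) mesh components.
; On BeginPlay it hides the currently unused second-magazine bone on both meshes.
; When the attachment replicates, it passes its per-magazine ammo count to the owner through a SetMagAmmo message.
; A helper function destroys the first-person component.
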(event EventBeginPlay
  ;[0 0 0] Begin Play
  (|CallParentFunction)
  (Components|SkinnedMesh|HideBonebyName (Variables|Default|GetFPP) "mag_02" "PBO_None") ; Hide second mag since it is not used for now.
)

(event EventOnAttachmentReplicated
  ;[0 0 0] Set Mag Ammo
  (Class|BIWeapon|SetMagAmmo(Message) (Components|GetOwner) (Variables|Capacity|GetAmmoPerMag)))

(fn ConstructionScript
  (|CallParentFunction))

(fn DestroyFPPComponent
  (Components|DestroyComponent (Variables|Default|GetFPP)))