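; BP_ClusterStrike is an actor that calls down a cluster of missiles around its location.
; On BeginPlay it shows a WB_ClusterStrike_Icon marker through Widget1, passing it the strike location, and removes that widget after a short delay.
; It spawns NumberOfMissiles BP_Missile actors high overhead with random horizontal scatter and its own Instigator.
; Each missile starts higher than the last, staggering the strike without timers.
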(event EventBeginPlay
  ;[0 0 0] Begin Play
  (bind _returnvalue (UserInterface|CreateWidget "/Game/FPS/UI/Gameplay/Widget_Icons/WB_ClusterStrike_Icon.WB_ClusterStrike_Icon_C"))
  (UserInterface|SetWidget (Variables|Default|GetWidget1) _returnvalue)
  (Variables|/Game/FPS/UI/Gameplay/Widget_Icons/WB_ClusterStrike_Icon.WB_ClusterStrike_Icon_C|SetObjetiveLocation _returnvalue (Transformation|GetActorLocation self))
  (for _index (range 0 (- (Variables|Default|GetNumberOfMissiles) 1)) ; Spawn Missiles
    (Game|SpawnActorfromClass "/Game/FPS/Blueprints/ClusterStrike/BP_Missile.BP_Missile_C" (Math|Transform|MakeTransform (+ (Transformation|GetActorLocation) (Math|Vector|MakeVector (Math|Random|RandomFloatinRange -4e+02 4e+02) (Math|Random|RandomFloatinRange -4e+02 4e+02) (+ 1e+04 (* _index 5000)))) "-90.000000,0.000000,0.000000" "1.000000,1.000000,1.000000") "Undefined" "MultiplyWithRoot" 0 (Game|GetInstigator)))
  (Utilities|FlowControl|Delay 4.0)
  (Components|DestroyComponent (Variables|Default|GetWidget1)))

(fn ConstructionScript)