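; BP_Missile is a Cluster Strike projectile that explodes on impact.
; On spawn it hides its mesh and waits InitialDelay, then shows the mesh and activates ProjectileMovement, allowing delayed launches.
; When the projectile stops, it spawns explosion effects and sound at the impact point and destroys only the mesh component.
; It then applies radial damage with the ClusterStrike damage type, credited to its instigator, and shakes nearby cameras.
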(event OnProjectileStop(ProjectileMovement)
  (params (ImpactResult :type Hit%20Result%20Structure%20%28by%20ref%29))
  (bind _impactpoint (Collision|BreakHitResult ImpactResult))
  ;[0 0 0] On stop movement
  (Effects|SpawnEmitteratLocation "/Game/FPS/Effects/WeaponEffects/Explosion/P_Explosion.P_Explosion" _impactpoint "0, 0, 0" "7.000000,7.000000,7.000000")
  (Audio|PlaySoundatLocation "/Game/FPS/Sound/Explosions/SC_Explosion_with_Metal_Debris.SC_Explosion_with_Metal_Debris" _impactpoint "0, 0, 0" 1.0 1.0 0.0 0 0 0 0)
  (Components|DestroyComponent (Variables|Default|GetStaticMesh))
  (Game|Damage|ApplyRadialDamage 2.5e+02 _impactpoint 1.2e+03 "/Game/FPS/Blueprints/Weapons/DamageTypes/DT_ClusterStrike.DT_ClusterStrike_C" 0 self (Game|GetInstigatorController) false "ECC_Visibility")
  (Camera|PlayWorldCameraShake "/Game/FPS/Blueprints/CameraShake/CS_Explosion.CS_Explosion_C" _impactpoint 8e+02 2.5e+03 1.0 true))

(event EventBeginPlay
  (bind _staticmesh (Variables|Default|GetStaticMesh))
  ;[0 0 0 0.5] Begin Play
  (Rendering|SetVisibility _staticmesh false false)
  (Utilities|FlowControl|Delay (Variables|Default|GetInitial%20delay))
  (Rendering|SetVisibility _staticmesh true false)
  (Components|Activation|Activate (Variables|Default|GetProjectileMovement) false))

(fn ConstructionScript)